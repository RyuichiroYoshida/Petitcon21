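; BP_PushController is a Blueprint that lets the first-person character push a cube by bumping into it.
; Each component hit from the character nudges the cube horizontally away from them by a scaled-down offset between their positions, without sweeping for collisions.
; A DoOnce reset after a short delay throttles the stone-sliding sound played at the cube, while movement continues on every hit.
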(event OnComponentHit(Cube)
  (params (HitComponent :type Primitive%20Component%20Object%20Reference) (OtherActor :type Actor%20Object%20Reference) (OtherComp :type Primitive%20Component%20Object%20Reference) (NormalImpulse :type Vector :default "0, 0, 0") (Hit :type Hit%20Result%20Structure%20%28by%20ref%29))
  (bind _cube (Variables|Default|GetCube))
  (bind _returnvalue (Transformation|GetWorldLocation _cube))
  (bind _asbp_first_person_character (Utilities|Casting|CastToBP_FirstPersonCharacter OtherActor))
  (Transformation|AddWorldOffset (Variables|Default|GetCube) (Math|Vector|MakeVector (.X (Math|Vector|BreakVector (/ (- _returnvalue (Transformation|GetActorLocation _asbp_first_person_character)) "50.000000,50.000000,50.000000"))) (.Y (Math|Vector|BreakVector (/ (- _returnvalue (Transformation|GetActorLocation _asbp_first_person_character)) "50.000000,50.000000,50.000000"))) 0.0) false false)
  (Utilities|FlowControl|DoOnce false :!label _label
    (:Completed
      (Audio|PlaySoundatLocation "/Game/SE/石の壁がスライドする.石の壁がスライドする" _returnvalue "0, 0, 0" 1.0 1.0 0.0 0 0 0 0)
      (Utilities|FlowControl|Delay 1.5)
      (goto _label Reset))))

(fn ConstructionScript)