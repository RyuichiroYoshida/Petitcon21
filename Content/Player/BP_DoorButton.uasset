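; BP_DoorButton is a button the player can activate once to open a linked stone door.
; On ActionPick, a DoOnce gate triggers a camera shake on the first player's camera and calls DoorOpen on the referenced Door.
; Falling-pebble and sliding-stone-wall sounds play at the door's location rather than the button's.
; GetItemInfo returns the button's ST item info.
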(event EventActionPick
  (bind _door (Variables|Default|GetDoor))
  (bind _returnvalue (Transformation|GetActorLocation _door))
  (Utilities|FlowControl|DoOnce false
    (:Completed
      (CameraShakes|StartCameraShake (Game|GetPlayerCameraManager 0) "/Game/Player/BP_CameraShake.BP_CameraShake_C" 1.0 "CameraLocal" "0, 0, 0")
      (Default|DoorOpen _door)
      (Audio|PlaySoundatLocation "/Game/SE/崖から石がパラパラ落ちる.崖から石がパラパラ落ちる" _returnvalue "0, 0, 0" 1.0 1.0 0.0 0 0 0 0)
      (Audio|PlaySoundatLocation "/Game/SE/石の壁がスライドする.石の壁がスライドする" _returnvalue "0, 0, 0" 1.0 1.0 0.0 0 0 0 0))))

(fn ConstructionScript)

(fn GetItemInfo
  (return (Variables|Default|GetST)))