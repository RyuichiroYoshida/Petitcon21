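; BP_GameManager is a Blueprint that drains a Fuel value and prints it as it falls.
; Five seconds after BeginPlay, a while loop calls FuelController until Fuel is no longer above zero.
; FuelController subtracts one and prints the value, which the loop then prints again.
; The loop has no delay inside, so the whole drain completes within a single frame.
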(event EventBeginPlay
  (Utilities|FlowControl|Delay 5.0)
  (while (< 0.0 (Variables|Default|GetFuel))
    (CallFunction|FuelController)
    (Development|PrintString (Utilities|String|ToString(Float) (Variables|Default|GetFuel)))))

(fn ConstructionScript)

(fn FuelController
  (bind _output_get (Variables|Default|SetFuel (- (Variables|Default|GetFuel) 1.0)))
  (Development|PrintString (Utilities|String|ToString(Float) _output_get)))