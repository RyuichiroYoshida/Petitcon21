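; BP_Door is a door Blueprint with a DoorOpen function that shifts the Door component to open it.
; DoorOpen adds MoveValue as a local offset in one unswept step, then prints a debug message.
; The DoorOpen call in the event graph is not triggered by any event, and a VInterpTo node for smooth movement toward a target height is left unused.
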(fn ConstructionScript)

(fn DoorOpen
  (Transformation|AddLocalOffset (Variables|Default|GetDoor) (Variables|Default|GetMoveValue) false false)
  (Development|PrintString "Finish Move"))